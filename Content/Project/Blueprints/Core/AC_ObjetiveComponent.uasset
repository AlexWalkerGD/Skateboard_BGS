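; Objective component that steps through an array of objectives and shows the current one on the skate HUD.
; BeginPlay spawns a W_Objetive widget for the next entry into the H_Skate HUD's vertical box.
; CompleteObjetive increments a counter, updates the widget's capped count, and plays its exit animation once the target is reached.
; RemoveWidget removes the widget and spawns the next; the counter is never reset here.
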(event `self.ReceiveBeginPlay`
  (`self.SpawnObjetive`))

(fn `CompleteObjetive`
  (bind _currentobjetive (`self.CurrentObjetive`))
  (bind _getout (`/Game/Project/UI/W_Objetive.GetOut` _currentobjetive))
  (bind _ntimes (`/Game/Project/Blueprints/Data/PDA_Objetive.nTimes` (`|GetArrayItem` (`self.Objetives`) (`self.IndexObjetive`))))
  (`/Engine/EditorBlueprintResources/StandardMacros.IncrementInt` (`self.nCount`)
    (:`  `
      (`/Game/Project/UI/W_Objetive.UpdateTimes` (`self.CurrentObjetive`) (`KismetMathLibrary.SelectInt` _ntimes (`self.nCount`) (> (`self.nCount`) _ntimes)))
      (if (>= (`self.nCount`) (`/Game/Project/Blueprints/Data/PDA_Objetive.nTimes` (`|GetArrayItem` (`self.Objetives`) (`self.IndexObjetive`))))
        (`Widget.SetVisibility` (`/Game/Project/UI/W_Objetive.Complete` (`self.CurrentObjetive`)) "Visible")
        (`UserWidget.PlayAnimation` _currentobjetive _getout 0.0 1 "Forward" 1.0 false)
        (`UserWidget.BindToAnimationFinished` _currentobjetive _getout (`|CreateDelegate` :!event `RemoveWidget`))))))

(fn `RemoveWidget`
  (`Widget.RemoveFromParent` (`self.CurrentObjetive`))
  (`self.SpawnObjetive`))

(fn `SpawnObjetive`
  (`/Engine/EditorBlueprintResources/StandardMacros.IncrementInt` (`self.IndexObjetive`)
    (:`  `
      (if (< (`self.IndexObjetive`) (`KismetArrayLibrary.Array_Length` (`self.Objetives`)))
        (bind _returnvalue (`|CreateWidget` "/Game/Project/UI/W_Objetive.W_Objetive_C" null (`|GetArrayItem` (`self.Objetives`) (`self.IndexObjetive`))))
        (set `self.CurrentObjetive` _returnvalue)
        (bind _ash_skate (cast `/Game/Project/Blueprints/Core/H_Skate` (`PlayerController.GetHUD` (`GameplayStatics.GetPlayerController` 0))))
        (`VerticalBox.AddChildToVerticalBox` (`/Game/Project/UI/W_HUD.SpaceToObjetive` (`/Game/Project/Blueprints/Core/H_Skate.WHUD` _ash_skate)) _returnvalue)))))