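; BFL_Library is a function library with lookup helpers for the score and objective components on an actor.
; FindScoreComponent and FindObjetiveComponent each take an Actor and fetch its AC_ScoreComponent or AC_ObjetiveComponent by class.
; Both validate the actor and the component, returning the component only when both checks pass and nothing otherwise.
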(fn `FindObjetiveComponent`
  (params (Actor :type "Actor Object Reference"))
  (returns (ObjetiveComponent :type "/Game/Project/Blueprints/Core/AC_ObjetiveComponent Object Reference"))
  (bind _returnvalue (`Actor.GetComponentByClass` Actor "/Game/Project/Blueprints/Core/AC_ObjetiveComponent.AC_ObjetiveComponent_C"))
  (`/Engine/EditorBlueprintResources/StandardMacros.IsValid` Actor
    (:`Is Valid`
      (`/Engine/EditorBlueprintResources/StandardMacros.IsValid` _returnvalue
        (:`Is Valid`
          (return _returnvalue))
        (:`Is Not Valid`
          (return null))))
    (:`Is Not Valid`
      (return null))))

(fn `FindScoreComponent`
  (params (Actor :type "Actor Object Reference"))
  (returns (ScoreComponent :type "/Game/Project/Blueprints/Core/AC_ScoreComponent Object Reference"))
  (bind _returnvalue (`Actor.GetComponentByClass` Actor "/Game/Project/Blueprints/Core/AC_ScoreComponent.AC_ScoreComponent_C"))
  (`/Engine/EditorBlueprintResources/StandardMacros.IsValid` Actor
    (:`Is Valid`
      (`/Engine/EditorBlueprintResources/StandardMacros.IsValid` _returnvalue
        (:`Is Valid`
          (return _returnvalue))
        (:`Is Not Valid`
          (return null))))
    (:`Is Not Valid`
      (return null))))