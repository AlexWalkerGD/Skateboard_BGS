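; Base pickup actor that triggers a speed change on the player when touched.
; It caches the BP_Player at BeginPlay, and a sphere collision checks overlapping actors for the "Player" tag.
; On a match it hands its float curve to the player for acceleration and deceleration, enables the player's speed-change flag, then expires via a very short lifespan.
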(event `self.ReceiveBeginPlay`
  (bind _asbp_player (cast `/Game/Project/Blueprints/Core/BP_Player` (`GameplayStatics.GetPlayerCharacter` 0)))
  (set `self.Player` _asbp_player))

(event `self.SphereCollision.OnComponentBeginOverlap`
  (params (OverlappedComponent :type "PrimitiveComponent Object Reference") (OtherActor :type "Actor Object Reference") (OtherComp :type "PrimitiveComponent Object Reference") (OtherBodyIndex :type Integer) (bFromSweep :type Boolean) (SweepResult :type "HitResult Structure (by ref)"))
  (bind _player (`self.Player`))
  (if (`self.ActorHasTag` OtherActor "Player")
    ;[0.05127 0.05127 0.05127] Set acceleration and deceleration
    (set `/Game/Project/Blueprints/Core/BP_Player.CurveFloat` (`self.CurveFloat`) _player)
    (set `/Game/Project/Blueprints/Core/BP_Player.CanChangeSpeed` true _player)
    (`self.SetLifeSpan` 0.1)))

(fn `UserConstructionScript`)