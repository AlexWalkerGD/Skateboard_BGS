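; Base skateboarding obstacle that rewards the player for clearing it and causes a wipeout on impact.
; Leaving the collision volume adds points through the player's score component, unless the obstacle has registered a hit.
; A hit detaches the skate, raises physics blend weight on player and skate meshes for a physics-driven fall, and unpossesses the player.
; After a short delay, respawning reopens the main map.
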(event `self.ObstacleCollision.OnComponentEndOverlap`
  (params (OverlappedComponent :type "PrimitiveComponent Object Reference") (OtherActor :type "Actor Object Reference") (OtherComp :type "PrimitiveComponent Object Reference") (OtherBodyIndex :type Integer))
  (if (`self.ActorHasTag` OtherActor "Player")
    (`self.CompletedObstacle` OtherActor (`self.Points`))))

(event `self.Obstacle.OnComponentHit`
  (params (HitComponent :type "PrimitiveComponent Object Reference") (OtherActor :type "Actor Object Reference") (OtherComp :type "PrimitiveComponent Object Reference") (NormalImpulse :type "Vector Structure") (Hit :type "HitResult Structure (by ref)"))
  (if (`self.ActorHasTag` OtherActor "Player")
    (set `self.PlayerHit` true)
    (bind _asbp_player (cast `/Game/Project/Blueprints/Core/BP_Player` OtherActor))
    (bind _success (`self.FailedObstacle` _asbp_player))
    (if _success
      (`KismetSystemLibrary.Delay` 2.0)
      (`self.RespawnPlayer`))))

(fn `CompletedObstacle`
  (params (Actor :type "Actor Object Reference") (Amount :type Integer))
  (bind _scorecomponent (`/Game/Project/Blueprints/Core/BFL_Library.FindScoreComponent` Actor))
  (if (not (`self.PlayerHit`))
    (`/Engine/EditorBlueprintResources/StandardMacros.IsValid` _scorecomponent
      (:`Is Valid`
        (`/Game/Project/Blueprints/Core/AC_ScoreComponent.IncreasePoints` _scorecomponent Amount)))))

(fn `FailedObstacle`
  (params (Player :type "/Game/Project/Blueprints/Core/BP_Player Object Reference"))
  (returns (Success :type Boolean))
  (`self.K2_DetachFromActor` (`/Game/Project/Blueprints/Core/BP_Player.Skate` Player) "KeepWorld" "KeepWorld" "KeepWorld")
  (`SkeletalMeshComponent.SetPhysicsBlendWeight` (`Character.Mesh` Player) 1.0)
  (`SkeletalMeshComponent.SetPhysicsBlendWeight` (`/Game/Project/Blueprints/Items/BP_Skate.Skate` (`/Game/Project/Blueprints/Core/BP_Player.Skate` Player)) 1.0)
  (`Controller.UnPossess` (`Pawn.GetController` Player))
  (return true))

(fn `RespawnPlayer`
  (locals (Location :type "Vector Structure" :default (0.0 0.0 0.0)))
  (`GameplayStatics.OpenLevel` "MainMap"))

(fn `UserConstructionScript`)